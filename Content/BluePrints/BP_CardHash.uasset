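; BP_CardHash is the card registry, bucketing cards by type and tracking how many the player has seen.
; BeginPlay spawns one BP_CardCollectionbyCardType per type, and AddCard files cards into them.
; AddCard also records next-card indices from type-one Yes/No functions, so random draws (by type, any, or excluding a type) pick only unseen, non-follow-up cards.
; It also exports and restores its state and each collection's as save data.
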(event `self.ReceiveBeginPlay`
  ;[1 1 1] 0. BeginPlay
  (`KismetArrayLibrary.Array_Clear` (`self.NextCardIndexArr`))
  (`KismetArrayLibrary.Array_Clear` (`self.CardHashArr`))
  (for _index (range (`self.NumOfCardType`))
    (bind _returnvalue (`|SpawnActorFromClass` "/Game/BluePrints/BP_CardCollectionbyCardType.BP_CardCollectionbyCardType_C" (`KismetMathLibrary.MakeTransform` (0.0 0.0 0.0)) "AlwaysSpawn" "OverrideRootScale" null _index null))
    (`KismetArrayLibrary.Array_Add` (`self.CardHashArr`) _returnvalue)))

(fn `AddCard`
  (params (NewCard :type "/Game/Struct/MyCardInfo_Struct Structure"))
  (returns (`Success?` :type Boolean))
  (locals (local_newCard :type "/Game/Struct/MyCardInfo_Struct Structure") (`local_Success?` :type Boolean))
  (set `local.local_newCard` NewCard)
  (set `local.local_Success?` false)
  (for _array_element (`self.CardHashArr`)
    (if (`|EnumEquality` (`.E_CardType_21_FABABC944A66AAC4195078B26DC31B47` (break `/Game/Struct/MyCardInfo_Struct` (`local.local_newCard`))) (`/Game/BluePrints/BP_CardCollectionbyCardType.E_CardType` _array_element))
      ;[0.7372 1 0.01217] 카드의 내용에 함수의 타입이 1이 있는지 확인 후에 따로 저장
      (`self.SetNextCardIndexArr` (`local.local_newCard`))
      (`/Game/BluePrints/BP_CardCollectionbyCardType.AddCardInArr` _array_element (`local.local_newCard`))
      (set `local.local_Success?` true)
      (break)))
  (return (`local.local_Success?`)))

(fn `CheckCardIdxWhenFuncTypeOne`
  (params (CardDataTableIdx :type Integer))
  (returns (UseOK :type Boolean))
  (return (== (`KismetArrayLibrary.Array_Find` (`self.NextCardIndexArr`) CardDataTableIdx) -1)))

(fn `CheckEndOfCard?`
  (returns (EndOfCard :type Boolean))
  (return (>= (`self.NumOfSeenByUser`) (`self.NumOfTotalCard`))))

(fn `GetCardByCardTypeWithOutNext`
  (params (CardType :type "/Game/Enum/E_CardType Enum" :default "NewEnumerator0"))
  (returns (`FoundCard?` :type Boolean) (Card :type "/Game/Struct/MyCardInfo_Struct Structure"))
  (locals (local_CardType :type "/Game/Enum/E_CardType Enum") (local_CardActor :type "/Game/BluePrints/BP_CardCollectionbyCardType Object Reference") (l_SelectableCardIdxArr :type "Array of Integer") (l_CntSelectableCardIdxArr :type Integer))
  (bind _allselectablecardsidx (`/Game/BluePrints/BP_CardCollectionbyCardType.GetAllSelectAbleCardsIdx` (`local.local_CardActor`) (`self.NextCardIndexArr`)))
  (set `local.local_CardType` CardType)
  (set `local.local_CardActor` null) ; null
  (for _array_element (`self.CardHashArr`)
    (if (`|EnumEquality` (`/Game/BluePrints/BP_CardCollectionbyCardType.E_CardType` _array_element) (`local.local_CardType`))
      (set `local.local_CardActor` _array_element)
      (break)))
  (`/Engine/EditorBlueprintResources/StandardMacros.IsValid` (`local.local_CardActor`)
    (:`Is Valid`
      (`KismetArrayLibrary.Array_Clear` (`local.l_SelectableCardIdxArr`))
      ;[1 1 1] 카드를 찾는 조건은, 아직 보여지지 않은 카드이면서 해당 카드가 다음인덱스에 영향을 주는 카드가 아니어야 한다.
      (if (> (`KismetArrayLibrary.Array_Length` _allselectablecardsidx) 0)
        (`KismetArrayLibrary.Array_Append` (`local.l_SelectableCardIdxArr`) _allselectablecardsidx)
        (set `local.l_CntSelectableCardIdxArr` (`KismetArrayLibrary.Array_Length` (`local.l_SelectableCardIdxArr`)))
        (if (> (`local.l_CntSelectableCardIdxArr`) 0)
          (bind (_foundcard_ _card) (`self.GetCardByDataTableIdx` (`|GetArrayItem` (`local.l_SelectableCardIdxArr`) (`KismetMathLibrary.RandomIntegerInRange` 0 (- (`local.l_CntSelectableCardIdxArr`) 1)))))
          (return _foundcard_ _card)
          (else
            (return false) ; 조건을 만족하는 카드가 없다
          ))
        (else
          (return false))))
    (:`Is Not Valid`
      (return false))))

(fn `GetCardByDataTableIdx`
  (params (DataTableIndex :type Integer))
  (returns (`FoundCard?` :type Boolean) (Card :type "/Game/Struct/MyCardInfo_Struct Structure"))
  (locals (`local_FoundCard?` :type Boolean) (local_Index :type Integer) (local_Card :type "/Game/Struct/MyCardInfo_Struct Structure"))
  (set `local.local_Index` DataTableIndex)
  (set `local.local_FoundCard?` false)
  (for _array_element (`self.CardHashArr`)
    (bind (_foundcard_ _card) (`/Game/BluePrints/BP_CardCollectionbyCardType.GetCardCorespondingIdx` _array_element (`local.local_Index`)))
    (if _foundcard_
      (set `local.local_FoundCard?` true)
      (set `local.local_Card` _card)
      (break)))
  (return (`local.local_FoundCard?`) (`local.local_Card`)))

(fn `GetCardByRandomWithOutNext`
  (returns (`FoundCard?` :type Boolean) (Card :type "/Game/Struct/MyCardInfo_Struct Structure"))
  (locals (l_SelectableCardIdxArr :type "Array of Integer") (l_CntSelectableCardIdxArr :type Integer))
  (`KismetArrayLibrary.Array_Clear` (`local.l_SelectableCardIdxArr`))
  (for _array_element (`self.CardHashArr`)
    (bind _allselectablecardsidx (`/Game/BluePrints/BP_CardCollectionbyCardType.GetAllSelectAbleCardsIdx` _array_element (`self.NextCardIndexArr`)))
    (if (> (`KismetArrayLibrary.Array_Length` _allselectablecardsidx) 0)
      (`KismetArrayLibrary.Array_Append` (`local.l_SelectableCardIdxArr`) _allselectablecardsidx)))
  (set `local.l_CntSelectableCardIdxArr` (`KismetArrayLibrary.Array_Length` (`local.l_SelectableCardIdxArr`)))
  (if (> (`local.l_CntSelectableCardIdxArr`) 0)
    (bind (_foundcard_ _card) (`self.GetCardByDataTableIdx` (`|GetArrayItem` (`local.l_SelectableCardIdxArr`) (`KismetMathLibrary.RandomIntegerInRange` 0 (- (`local.l_CntSelectableCardIdxArr`) 1)))))
    (return _foundcard_ _card)
    (else
      (return false))))

(fn `GetCardExceptionCardTypeWithOutNext`
  (params (ExceptionCardType :type "/Game/Enum/E_CardType Enum" :default "NewEnumerator0"))
  (returns (`FoundCard?` :type Boolean) (Card :type "/Game/Struct/MyCardInfo_Struct Structure"))
  (locals (local_ExceptionCardType :type "/Game/Enum/E_CardType Enum") (l_SelectableCardIdxArr :type "Array of Integer") (l_CntSelectableCardIdxArr :type Integer))
  (set `local.local_ExceptionCardType` ExceptionCardType)
  (`KismetArrayLibrary.Array_Clear` (`local.l_SelectableCardIdxArr`))
  (for _array_element (`self.CardHashArr`)
    (if (`|EnumInequality` (`/Game/BluePrints/BP_CardCollectionbyCardType.E_CardType` _array_element) (`local.local_ExceptionCardType`))
      (bind _allselectablecardsidx (`/Game/BluePrints/BP_CardCollectionbyCardType.GetAllSelectAbleCardsIdx` _array_element (`self.NextCardIndexArr`)))
      ;[1 1 1] Length가 0이든 0이아니든 상관없이 Append해도 상관없을 듯?
      (if (> (`KismetArrayLibrary.Array_Length` _allselectablecardsidx) 0)
        (`KismetArrayLibrary.Array_Append` (`local.l_SelectableCardIdxArr`) _allselectablecardsidx))))
  (set `local.l_CntSelectableCardIdxArr` (`KismetArrayLibrary.Array_Length` (`local.l_SelectableCardIdxArr`)))
  (if (> (`local.l_CntSelectableCardIdxArr`) 0)
    (bind (_foundcard_ _card) (`self.GetCardByDataTableIdx` (`|GetArrayItem` (`local.l_SelectableCardIdxArr`) (`KismetMathLibrary.RandomIntegerInRange` 0 (- (`local.l_CntSelectableCardIdxArr`) 1)))))
    (return _foundcard_ _card)
    (else
      (return false))))

(fn `GetCardHashArrLen`
  (returns (Len :type Integer))
  (return (`KismetArrayLibrary.Array_Length` (`self.CardHashArr`))))

(fn `GetNumOfTotalCard`
  (returns (NumOfTotalCard :type Integer))
  (return (`self.NumOfTotalCard`)))

(fn `GetRandomCard`
  (returns (FoundCard :type Boolean) (Card :type "/Game/Struct/MyCardInfo_Struct Structure"))
  (locals (Local_CardIndex :type Integer) (`local_FoundCard?` :type Boolean) (local_Card :type "/Game/Struct/MyCardInfo_Struct Structure"))
  (set `local.local_FoundCard?` false)
  (for _array_element (`self.CardHashArr`)
    (set `local.Local_CardIndex` (`KismetMathLibrary.RandomIntegerInRange` 0 (- (`self.NumOfTotalCard`) 1)))
    (bind (_foundcard_ _card) (`/Game/BluePrints/BP_CardCollectionbyCardType.GetCardCorespondingIdx` _array_element (`local.Local_CardIndex`)))
    (if _foundcard_
      (set `local.local_FoundCard?` true)
      (set `local.local_Card` _card)
      (break)))
  (if (`local.local_FoundCard?`)
    (return (`local.local_FoundCard?`) (`local.local_Card`))
    (else
      (`KismetSystemLibrary.PrintString` "Hello"))))

(fn `GetSaveCardHashData`
  (returns (DataToSave :type "/Game/SaveGame/CardHashStruct Structure"))
  (locals (local_SaveData :type "/Game/SaveGame/CardHashStruct Structure") (local_initArr :type "Array of /Game/SaveGame/EachTypeCardArrStruct Structure"))
  (bind (_numofcardtype _functiontypeone _numoftotalcard _numofseenbyuser _nextcardindexarr _eachtypecardarrstruct) (break `/Game/SaveGame/CardHashStruct` (`local.local_SaveData`)))
  (`KismetArrayLibrary.Array_Clear` (`local.local_initArr`))
  (set `local.local_SaveData` (make `/Game/SaveGame/CardHashStruct` (`self.NumOfCardType`) (`self.FunctionTypeOne`) (`self.NumOfTotalCard`) (`self.NumOfSeenByUser`) (`self.NextCardIndexArr`) (`local.local_initArr`)))
  (for _array_element (`self.CardHashArr`)
    (bind _datatosave (`/Game/BluePrints/BP_CardCollectionbyCardType.GetSaveData` _array_element))
    (`KismetArrayLibrary.Array_Add` (`.EachTypeCardArrStruct_4_6D0B7E5748FB89A8C68DA6AB1D18AC6D` (break `/Game/SaveGame/CardHashStruct` (`local.local_SaveData`))) _datatosave))
  ;[0 1 0.256] Debug
  (`KismetSystemLibrary.PrintString` (`KismetStringLibrary.Conv_IntToString` (`KismetArrayLibrary.Array_Length` _eachtypecardarrstruct)))
  (for _array_element_2 _eachtypecardarrstruct
    (bind (_cardtypeininteger _e_cardtype _cardcollection) (break `/Game/SaveGame/EachTypeCardArrStruct` _array_element_2))
    (`/Game/SaveGame/OnlyForDebugging.ShowDebugCardHashArrData` _cardtypeininteger _e_cardtype _cardcollection))
  (return (`local.local_SaveData`)))

(fn `SetIsSeen`
  (params (CardType :type "/Game/Enum/E_CardType Enum" :default "NewEnumerator0") (Index :type Integer) (IsSeen :type Boolean))
  (returns (`Success?` :type Boolean) (NumOfSeenByUser :type Integer))
  (locals (local_CardType :type "/Game/Enum/E_CardType Enum") (local_Index :type Integer))
  (set `local.local_CardType` CardType)
  (set `local.local_Index` Index)
  (for _array_element (`self.CardHashArr`)
    (if (`|EnumEquality` (`local.local_CardType`) (`/Game/BluePrints/BP_CardCollectionbyCardType.E_CardType` _array_element))
      (bind _success_ (`/Game/BluePrints/BP_CardCollectionbyCardType.SetIsSeen` _array_element (`local.local_Index`) IsSeen))
      (if _success_
        (set `self.NumOfSeenByUser` (+ (`self.NumOfSeenByUser`) 1))
        (return true (`self.NumOfSeenByUser`))
        (else
          (return false (`self.NumOfSeenByUser`))))))
  (return false (`self.NumOfSeenByUser`)))

(fn `SetNextCardIndexArr`
  (params (Card :type "/Game/Struct/MyCardInfo_Struct Structure"))
  (locals (local_Yes_FuncType :type Integer) (local_No_FuncType :type Integer) (local_Card :type "/Game/Struct/MyCardInfo_Struct Structure"))
  (set `local.local_Card` Card)
  ;[1 1 1] 함수의 타입들을 가지고 온다.
  (set `local.local_Yes_FuncType` (`.WHEN_FUNCTION_TYPE_2_6C47C52A49BD071D8D2391878556ACBB` (break `/Game/Struct/ClickButtonInfo_Struct` (`.YES_BUTTON_INFO_42_A831EA3D4B6A9B6361BEC2B7931F6D3B` (break `/Game/Struct/MyCardInfo_Struct` (`local.local_Card`))))))
  (set `local.local_No_FuncType` (`.WHEN_FUNCTION_TYPE_2_6C47C52A49BD071D8D2391878556ACBB` (break `/Game/Struct/ClickButtonInfo_Struct` (`.NO_BUTTON_INFO_43_5717935841A7E7BD88730EBA821F838F` (break `/Game/Struct/MyCardInfo_Struct` (`local.local_Card`))))))
  (`|ExecutionSequence`
    (:`then_0`
      ;[1 1 1] YES버튼 확인
      (if (== (`local.local_Yes_FuncType`) (`self.FunctionTypeOne`))
        (`KismetArrayLibrary.Array_Add` (`self.NextCardIndexArr`) (`.WHEN_FUNCTION_1_NEXT_IDX_4_05BD44F04EC785D4361D84807D9C1D3F` (break `/Game/Struct/ClickButtonInfo_Struct` (`.YES_BUTTON_INFO_42_A831EA3D4B6A9B6361BEC2B7931F6D3B` (break `/Game/Struct/MyCardInfo_Struct` (`local.local_Card`))))))))
    (:`then_1`
      ;[1 1 1] NO버튼 학인
      (if (== (`local.local_No_FuncType`) (`self.FunctionTypeOne`))
        (`KismetArrayLibrary.Array_Add` (`self.NextCardIndexArr`) (`.WHEN_FUNCTION_1_NEXT_IDX_4_05BD44F04EC785D4361D84807D9C1D3F` (break `/Game/Struct/ClickButtonInfo_Struct` (`.NO_BUTTON_INFO_43_5717935841A7E7BD88730EBA821F838F` (break `/Game/Struct/MyCardInfo_Struct` (`local.local_Card`))))))))))

(fn `SetNumOfTotalCard`
  (params (NumOfTotalCard :type Integer))
  (set `self.NumOfTotalCard` NumOfTotalCard))

(fn `SetSaveCardHashData`
  (params (SaveData :type "/Game/SaveGame/CardHashStruct Structure"))
  (locals (local_SaveData :type "/Game/SaveGame/CardHashStruct Structure") (local_SaveOKCountDEBUG :type Integer))
  (bind (_numofcardtype _functiontypeone _numoftotalcard _numofseenbyuser _nextcardindexarr) (break `/Game/SaveGame/CardHashStruct` (`local.local_SaveData`)))
  (set `local.local_SaveData` SaveData)
  (set `self.NumOfCardType` _numofcardtype)
  (set `self.FunctionTypeOne` _functiontypeone)
  (set `self.NumOfTotalCard` _numoftotalcard)
  (set `self.NumOfSeenByUser` _numofseenbyuser)
  (set `self.NextCardIndexArr` _nextcardindexarr)
  (`KismetSystemLibrary.PrintString` (`KismetStringLibrary.Conv_IntToString` (`KismetArrayLibrary.Array_Length` (`self.CardHashArr`))))
  (for _array_element (`self.CardHashArr`)
    (bind _saveok (`/Game/BluePrints/BP_CardCollectionbyCardType.SetSaveData` _array_element (`.EachTypeCardArrStruct_4_6D0B7E5748FB89A8C68DA6AB1D18AC6D` (break `/Game/SaveGame/CardHashStruct` (`local.local_SaveData`)))))
    (if _saveok
      (set `local.local_SaveOKCountDEBUG` (+ (`local.local_SaveOKCountDEBUG`) 1))))
  (if (== (`self.NumOfCardType`) (`local.local_SaveOKCountDEBUG`))
    (`KismetSystemLibrary.PrintString` "카드 타입만큼 데이터 세이브 Ok")
    (else
      (`KismetSystemLibrary.PrintString` "로드 시 에러 가능성 높음"))))

(fn `UserConstructionScript`)