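; BP_CardCollectionbyCardType holds the cards of one card type and tracks which have been seen.
; BeginPlay empties the collection and derives the card type enum from CardTypeInInteger.
; Functions add cards, find unseen ones by data-table index, set seen flags and list selectable indices minus an exclusion list.
; Save data packs type and collection, and loading restores the collection from the entry with the matching type.
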(event `self.ReceiveBeginPlay`
  ;[1 1 1] 0. BeginPlay
  (`KismetArrayLibrary.Array_Clear` (`self.CardCollection`))
  (set `self.E_CardType` (cast `/Game/Enum/E_CardType` (`KismetMathLibrary.Conv_IntToByte` (`self.CardTypeInInteger`)))))

(fn `AddCardInArr`
  (params (NewCard :type "/Game/Struct/MyCardInfo_Struct Structure"))
  (`KismetArrayLibrary.Array_Add` (`self.CardCollection`) NewCard)
  (return))

(fn `GetAllSelectAbleCardsIdx`
  (params (IdxsToWithOut :type "Array of Integer"))
  (returns (AllSelectAbleCardsIdx :type "Array of Integer"))
  (locals (local_AllSelectAbleCardsIdx :type "Array of Integer"))
  (`KismetArrayLibrary.Array_Clear` (`local.local_AllSelectAbleCardsIdx`))
  (for _array_element (`self.CardCollection`)
    (bind (_arridxindatatable _day _content _isseen_) (break `/Game/Struct/MyCardInfo_Struct` _array_element))
    (if (not _isseen_)
      (if (== (`KismetArrayLibrary.Array_Find` IdxsToWithOut _arridxindatatable) -1)
        (`KismetArrayLibrary.Array_Add` (`local.local_AllSelectAbleCardsIdx`) _arridxindatatable))))
  (return (`local.local_AllSelectAbleCardsIdx`)))

(fn `GetCardCorespondingIdx`
  (params (Index :type Integer))
  (returns (`FoundCard?` :type Boolean) (Card :type "/Game/Struct/MyCardInfo_Struct Structure"))
  (locals (local_Index :type Integer) (`local_FoundCard?` :type Boolean) (local_Card :type "/Game/Struct/MyCardInfo_Struct Structure"))
  (set `local.local_Index` Index)
  (set `local.local_FoundCard?` false)
  (for _array_element (`self.CardCollection`)
    (bind (_arridxindatatable _day _content _isseen_) (break `/Game/Struct/MyCardInfo_Struct` _array_element))
    (if (and (== (`local.local_Index`) _arridxindatatable) (not _isseen_))
      (set `local.local_FoundCard?` true)
      (set `local.local_Card` _array_element)
      (break)))
  (return (`local.local_FoundCard?`) (`local.local_Card`)))

(fn `GetSaveData`
  (returns (DataToSave :type "/Game/SaveGame/EachTypeCardArrStruct Structure"))
  (locals (local_SaveData :type "/Game/SaveGame/EachTypeCardArrStruct Structure"))
  (set `local.local_SaveData` (make `/Game/SaveGame/EachTypeCardArrStruct` (`self.CardTypeInInteger`) (`self.E_CardType`) (`self.CardCollection`)))
  (return (`local.local_SaveData`)))

(fn `SetIsSeen`
  (params (Index :type Integer) (IsSeen :type Boolean))
  (returns (`Success?` :type Boolean))
  (locals (local_Success :type Boolean))
  (set `local.local_Success` false)
  (for (_array_element _array_index) (`self.CardCollection`)
    (if (== Index (`.ArrIdxInDataTable_8_5F63F76B4DF6D3AB49E631ABEA866A2B` (break `/Game/Struct/MyCardInfo_Struct` _array_element)))
      (bind (_arridxindatatable _day _content _isseen_ _e_cardtype _yes_button_info _no_button_info) (break `/Game/Struct/MyCardInfo_Struct` _array_element))
      (`KismetArrayLibrary.Array_Set` (`self.CardCollection`) _array_index (make `/Game/Struct/MyCardInfo_Struct` _arridxindatatable _day _content IsSeen _e_cardtype _yes_button_info _no_button_info))
      (set `local.local_Success` true)
      (break)))
  (return (`local.local_Success`)))

(fn `SetSaveData`
  (params (SaveData :type "Array of /Game/SaveGame/EachTypeCardArrStruct Structure"))
  (returns (SaveOK :type Boolean))
  (locals (`local_SaveDataFound?` :type Boolean) (local_SaveData :type "Array of /Game/Struct/MyCardInfo_Struct Structure"))
  (`KismetArrayLibrary.Array_Clear` (`local.local_SaveData`))
  (set `local.local_SaveDataFound?` false)
  (for _array_element SaveData
    (bind (_cardtypeininteger _e_cardtype _cardcollection) (break `/Game/SaveGame/EachTypeCardArrStruct` _array_element))
    (if (`|EnumEquality` (`self.E_CardType`) _e_cardtype)
      (set `local.local_SaveDataFound?` true)
      (set `local.local_SaveData` _cardcollection)
      (break)))
  (if (`local.local_SaveDataFound?`)
    (set `self.CardCollection` (`local.local_SaveData`)))
  (return (`local.local_SaveDataFound?`)))

(fn `UserConstructionScript`)